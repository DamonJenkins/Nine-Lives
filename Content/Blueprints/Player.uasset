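; Player pawn for cursor-driven interaction: it possesses itself on BeginPlay, shows the mouse, and caches the level's Cat actor.
; The Rotate axis yaws its static mesh.
; Tick traces under the cursor and tracks LastHit to send hover and leave calls to Interactable actors, with OnMouseOver repeating every frame.
; Pressing Interact traces again and calls Interact on the hit Interactable, passing it the Cat.
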(event EventBeginPlay
  (bind _returnvalue (Game|GetPlayerController 0))
  (bind _returnvalue_2 (Actor|GetActorOfClass "/Game/Blueprints/Cat.Cat_C"))
  (Variables|Default|Setcat _returnvalue_2)
  (Pawn|Possess _returnvalue self)
  (Variables|/Script/Engine.PlayerController|SetbShowMouseCursor _returnvalue true)
  (Input|SetInputModeGameandUI _returnvalue 0 "DoNotLock" true))

(event Collision|EventActorBeginOverlap
  (params (OtherActor :type Actor%20Object%20Reference)))

(event EventTick
  (params (DeltaSeconds :type Float%20%28single-precision%29))
  (bind _returnvalue (Game|GetPlayerController 0))
  (bind (_hitresult _returnvalue_2) (Game|Player|GetHitResultUnderCursorbyChannel _returnvalue "TraceTypeQuery1" true))
  (if (!= (.hitactor _hitresult) 0)
    (bind _asinteractable (Utilities|Casting|CastToInteractable (.hitactor _hitresult))
      (:then
        _)
      (:CastFailed
        _))
    (if (and (!= _asinteractable (Variables|Default|GetlastHit)) (!= (Variables|Default|GetlastHit) 0))
      (bind _asinteractable_2 (Utilities|Casting|CastToInteractable (Variables|Default|GetlastHit))
        (:then
          (Default|OnMouseLeave _asinteractable_2))
        (:CastFailed
          _))
      (Variables|Default|SetlastHit _asinteractable :!label _label))
    (else
      (goto _label)))
  (if _returnvalue_2
    (bind _asinteractable_3 (Utilities|Casting|CastToInteractable (.hitactor _hitresult)))
    (Default|OnMouseOver _asinteractable_3)
    (Variables|Default|SetlastHit _asinteractable_3)))

(event Input|ActionEvents|InputActionInteract
  (params (Key :type Key%20Structure :default "None"))
  (bind _returnvalue (Game|GetPlayerController 0))
  (bind (_hitresult _returnvalue_2) (Game|Player|GetHitResultUnderCursorbyChannel _returnvalue "TraceTypeQuery1" true))
  (:Pressed
    (if _returnvalue_2
      (bind _asinteractable (Utilities|Casting|CastToInteractable (.hitactor _hitresult)))
      (Default|Interact _asinteractable (Variables|Default|Getcat)))))

(event Input|AxisEvents|InputAxisRotate
  (params (AxisValue :type Float%20%28single-precision%29))
  (Transformation|AddLocalRotation (Variables|Default|GetStaticMesh) (Math|Rotator|MakeRotator 0.0 0.0 AxisValue) false false))

(fn ConstructionScript)