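; Attractor is an interactable Blueprint that pulls cats toward itself when triggered.
; Its Interact event calls Attract on the passed Cat with hurting enabled, then on the EnemyCat if that reference is valid, without setting the hurt flag.
; Both calls target the static mesh's world location plus an offset and share the same Force magnitude.
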(event EventBeginPlay
  (|CallParentFunction) ; This node is disabled and will not be called.\nDrag off pins to build functionality.
)

(event Collision|EventActorBeginOverlap
  (params (OtherActor :type Actor%20Object%20Reference))
  (|CallParentFunction OtherActor) ; This node is disabled and will not be called.\nDrag off pins to build functionality.
)

(event EventTick
  (params (DeltaSeconds :type Float%20%28single-precision%29))
  (|CallParentFunction DeltaSeconds) ; This node is disabled and will not be called.\nDrag off pins to build functionality.
)

(event EventInteract
  (params (Cat :type Cat%20Object%20Reference) (EnemyCat :type Enemy%20Cat%20Object%20Reference))
  (bind _force (Variables|Default|Getforce))
  (bind _locationoffset (Variables|Default|GetLocationOffset))
  (bind _staticmesh (Variables|Default|GetStaticMesh))
  (bind _returnvalue (Transformation|GetWorldLocation _staticmesh))
  (bind _returnvalue_2 (+ _returnvalue _locationoffset))
  (Default|Attract Cat _returnvalue_2 _force true)
  (Utilities|IsValid EnemyCat
    (:Is%20Valid
      (Default|Attract EnemyCat _returnvalue_2 _force))))

(fn ConstructionScript
  (|CallParentFunction))