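; AirCon is an interactable air-conditioner actor that, when switched on, shoves the cat away without hurting it.
; Interact stores the cat and uses a FlipFlop to drive four air particle systems and the Attracting flag.
; While that flag is set, Tick calls the cat's Repel from the mesh position whenever the cat is within the distance threshold.
; Mouse hover swaps the mesh to a rim-highlight material.
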(event EventBeginPlay
  (|CallParentFunction) ; This node is disabled and will not be called.\nDrag off pins to build functionality.
)

(event Collision|EventActorBeginOverlap
  (params (OtherActor :type Actor%20Object%20Reference))
  (|CallParentFunction OtherActor) ; This node is disabled and will not be called.\nDrag off pins to build functionality.
)

(event EventTick
  (params (DeltaSeconds :type Float%20%28single-precision%29))
  (|CallParentFunction DeltaSeconds)
  (if (Variables|Default|GetAttracting)
    (if (< (|DistanceFromCat_2) (Variables|Default|GetDistanceThreshold))
      (Default|Repel (Variables|Default|GetTheCat) (|Position_2) (Variables|Default|GetShoveForce) false))))

(event EventOnMouseOver
  (Rendering|Material|SetMaterial (Variables|Default|GetStaticMesh) 0 "/Game/Assets/Models/rimblue.rimblue"))

(event EventOnMouseLeave
  (Rendering|Material|SetMaterial (Variables|Default|GetStaticMesh) 0 "/Game/Assets/Materials/Heater_M.Heater_M"))

(event EventInteract
  (params (Cat :type Cat%20Object%20Reference))
  (Variables|Default|SetTheCat Cat)
  (bind _isa (Utilities|FlowControl|FlipFlop)
    (:A
      (|FlipFlopParticleSystems :!label _label
        (:AOut
          _)
        (:BOut
          _))
      (Variables|Default|SetAttracting _isa))
    (:B
      (goto _label B))))

(fn ConstructionScript
  (|CallParentFunction))