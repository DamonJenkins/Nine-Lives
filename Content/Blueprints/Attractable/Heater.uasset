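; Interactable heater that toggles on and off and, while on, harmlessly tugs the cat toward it when within a distance threshold.
; Interact flips the attracting state, a cube's visibility and five particle systems, recording the toggle time.
; Tick drives the mesh's colour parameter from up/down curves, clamped component-wise against the current colour for one-way fades.
; Mouse hover swaps the mesh to a blue rim material.
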(event EventBeginPlay
  (|CallParentFunction) ; This node is disabled and will not be called.\nDrag off pins to build functionality.
)

(event Collision|EventActorBeginOverlap
  (params (OtherActor :type Actor%20Object%20Reference))
  (|CallParentFunction OtherActor) ; This node is disabled and will not be called.\nDrag off pins to build functionality.
)

(event EventTick
  (params (DeltaSeconds :type Float%20%28single-precision%29))
  (|CallParentFunction DeltaSeconds)
  (if (Variables|Default|GetAttracting)
    (Utilities|FlowControl|Sequence
      (:then_0
        (if (< (|DistanceFromCat) (Variables|Default|GetDistanceThreshold))
          (Default|Attract (Variables|Default|GetTheCat) (|Position) (Variables|Default|GetTugForce) false)))
      (:then_1
        (bind _output_get (Variables|Default|Setcurrent%20heater%20colour (Math|Vector|VectorComponentMax (Math|Conversions|ToVector(LinearColor) (Math|Curves|GetLinearColorValue (Variables|Default|GetColourUp) (- (Utilities|Time|GetTimeSeconds) (Variables|Default|Getactivation%20time)))) (Variables|Default|Getcurrent%20heater%20colour))))
        (Rendering|Material|SetVectorParameterValueonMaterials (Variables|Default|GetStaticMesh) "Colour_2" _output_get)))
    (else
      (bind _output_get_2 (Variables|Default|Setcurrent%20heater%20colour (Math|Vector|VectorComponentMin (Math|Conversions|ToVector(LinearColor) (Math|Curves|GetLinearColorValue (Variables|Default|GetColourDown) (- (Utilities|Time|GetTimeSeconds) (Variables|Default|Getactivation%20time)))) (Variables|Default|Getcurrent%20heater%20colour))))
      (Rendering|Material|SetVectorParameterValueonMaterials (Variables|Default|GetStaticMesh) "Colour_2" _output_get_2))))

(event EventOnMouseOver
  (Rendering|Material|SetMaterial (Variables|Default|GetStaticMesh) 0 "/Game/Assets/Models/rimblue.rimblue"))

(event EventOnMouseLeave
  (Rendering|Material|SetMaterial (Variables|Default|GetStaticMesh) 0 "/Game/Assets/Materials/NewMaterial_Inst.NewMaterial_Inst"))

(event EventInteract
  (params (Cat :type Cat%20Object%20Reference))
  (Variables|Default|SetTheCat Cat)
  (bind _isa (Utilities|FlowControl|FlipFlop)
    (:A
      _)
    (:B
      _))
  (Variables|Default|SetAttracting _isa)
  (Variables|Default|Setactivation%20time (Utilities|Time|GetTimeSeconds))
  (Rendering|SetVisibility (Variables|Default|GetCube) _isa false)
  (if _isa
    (Components|Activation|Activate (Variables|Default|GetParticleSystem2) false)
    (else
      (Components|Activation|Deactivate (Variables|Default|GetParticleSystem)))))

(fn ConstructionScript
  (|CallParentFunction))