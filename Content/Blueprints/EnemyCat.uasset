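; EnemyCat is a physics-driven cat enemy that can be pulled toward or pushed away from world locations.
; On BeginPlay, its Body simulates physics at full blend weight from the CatEnemySkeleton bone down, making it a ragdoll.
; Attract and Repel events apply a normalized horizontal force, scaled by the given magnitude, toward or away from the supplied location.
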(event Custom|Attract
  (params (WorldLocation :type Vector) (Magnitude :type Float%20%28single-precision%29))
  (bind _body (Variables|Default|GetBody))
  (bind _returnvalue (Transformation|GetWorldLocation _body))
  (bind _returnvalue_2 (- WorldLocation (Math|Vector|MakeVector (.x _returnvalue) (.y _returnvalue) 0.0)))
  (Physics|AddForce (Variables|Default|GetBody) (* (Math|Vector|Normalize (Math|Vector|MakeVector (.x _returnvalue_2) (.y _returnvalue_2) 0.0)) Magnitude) "None" false))

(event Custom|Repel
  (params (WorldLocation :type Vector) (Magnitude :type Float%20%28single-precision%29))
  (bind _body (Variables|Default|GetBody))
  (bind _returnvalue (Transformation|GetWorldLocation _body))
  (bind _returnvalue_2 (- _returnvalue WorldLocation))
  (Physics|AddForce (Variables|Default|GetBody) (* (Math|Vector|Normalize (Math|Vector|MakeVector (.x _returnvalue_2) (.y _returnvalue_2) 0.0)) Magnitude) "None" false))

(event EventBeginPlay
  (bind _returnvalue (Utilities|Name|MakeLiteralName "CatEnemySkeleton"))
  (bind _body (Variables|Default|GetBody))
  (Class|SkeletalMeshComponent|SetAllBodiesBelowSimulatePhysics _body _returnvalue true true)
  (Class|SkeletalMeshComponent|SetAllBodiesBelowPhysicsBlendWeight _body _returnvalue 1.0 false true))

(event Collision|EventActorBeginOverlap
  (params (OtherActor :type Actor%20Object%20Reference)))

(event EventTick
  (params (DeltaSeconds :type Float%20%28single-precision%29)))

(fn ConstructionScript)