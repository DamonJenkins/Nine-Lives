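; Game instance for the cat game that persists level progress and tracks the current score across levels.
; On Init it loads the GameSaveObject from its slot, or creates and saves a new one.
; SubmitLevelScore compares the score to saved bests and per-level thresholds, updates scores, unlocks the next level and returns a result enum plus an end-level flag.
; LoadLevel shows a loading-screen widget, records the played level and resets the score.
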(event EventInit
  (bind (_saveslotname _userindex) (Utilities|SaveInfo))
  (bind (_saveslotname_2 _userindex_2) (Utilities|SaveInfo))
  (bind _returnvalue (SaveGame|DoesSaveGameExist _saveslotname_2 _userindex_2))
  (if _returnvalue
    (bind _returnvalue_2 (SaveGame|LoadGamefromSlot _saveslotname _userindex))
    (bind _asgame_save_object (Utilities|Casting|CastToGameSaveObject _returnvalue_2))
    (Variables|Default|SetsaveObject _asgame_save_object)
    (else
      (bind _returnvalue_3 (SaveGame|CreateSaveGameObject "/Game/Blueprints/GameSaveObject.GameSaveObject_C"))
      (Variables|Default|SetsaveObject _returnvalue_3)
      (CallFunction|SaveGame))))

(fn GetScore
  (return (Variables|Default|Getscore)))

(fn ResetScore
  (Variables|Default|Setscore 0.0))

(fn SaveGame
  (bind (_outputpin _saveslotname _userindex) (|GetSaveInformation))
  (SaveGame|SaveGametoSlot _outputpin _saveslotname _userindex)
  (return))

(fn SubmitLevelScore
  (params (Score :type Float%20%28single-precision%29))
  (bind (_out _newhighscore) (|IsHighScore))
  (bind _saveobject (Variables|Default|GetsaveObject))
  (bind _playedlevel (Variables|Default|GetplayedLevel))
  (bind _playedlevel_2 (Variables|Default|GetplayedLevel))
  (bind _returnvalue (+ _playedlevel_2 1))
  (bind _levelsunlocked (Variables|/Game/Blueprints/GameSaveObject.GameSaveObject_C|GetLevelsUnlocked _saveobject))
  (bind _returnvalue_2 (Utilities|Array|Length _levelsunlocked))
  (bind _returnvalue_3 (> _returnvalue _returnvalue_2))
  (if _out
    (Utilities|Array|SetArrayElem (Variables|/Game/Blueprints/GameSaveObject.GameSaveObject_C|GetScores (Variables|Default|GetsaveObject)) (Variables|Default|GetplayedLevel) _newhighscore)
    (return "NewEnumerator4" _returnvalue_3)
    (elif (|LevelAlreadyCompleted)
      (return "NewEnumerator0" _returnvalue_3)
      (elif (|DidCompleteLevel)
        (Utilities|Array|SetArrayElem (Variables|/Game/Blueprints/GameSaveObject.GameSaveObject_C|GetScores (Variables|Default|GetsaveObject)) _playedlevel (Math|Float|Truncate (Variables|Default|Getscore)))
        (Utilities|Array|SetArrayElem (Variables|/Game/Blueprints/GameSaveObject.GameSaveObject_C|GetLevelsUnlocked (Variables|Default|GetsaveObject)) (+ _playedlevel 1) true)
        (return "NewEnumerator1" _returnvalue_3)
        (else
          (return "NewEnumerator2" _returnvalue_3))))))

(fn LoadLevel
  (params (Level :type Integer))
  (bind _returnvalue (UserInterface|CreateWidget "/Game/Blueprints/Widgets/LoadingScreen.LoadingScreen_C" (Game|GetPlayerController 0)))
  (bind _output_get (Variables|Default|SetloadWidget _returnvalue))
  (UserInterface|Viewport|AddtoViewport _output_get 0)
  (Variables|Default|SetplayedLevel (- Level 1))
  (Variables|Default|Setscore 0.0))

(fn LoadNextLevel
  (CallFunction|LoadLevel (+ (Variables|Default|GetplayedLevel) 2)))