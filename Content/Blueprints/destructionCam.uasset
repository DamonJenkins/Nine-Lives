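; Cinematic camera actor that gives a brief slow-motion view of a group of destructible objects.
; If its array starts empty, it gathers destructibles overlapping its Objects component, links itself to each, destroys that component and moves its root to their average location.
; SlowMoCam blends the player view to this actor under global time dilation, then after a short delay blends back to the Player actor and restores normal speed.
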(event Custom|SlowMoCam
  (Variables|Default|Setplaying true)
  (Game|Player|SetViewTargetwithBlend (Game|GetPlayerController 0) self 0.5 "VTBlend_EaseInOut" 2.0 false)
  (Utilities|Time|SetGlobalTimeDilation 0.3)
  (bind _returnvalue (Actor|GetActorOfClass "/Game/Blueprints/Player.Player_C"))
  (Utilities|FlowControl|Delay 0.51)
  (Game|Player|SetViewTargetwithBlend (Game|GetPlayerController 0) _returnvalue 1.0 "VTBlend_EaseInOut" 2.0 false)
  (Utilities|Time|SetGlobalTimeDilation 1.0))

(event Custom|populateArray
  (for _array_element (Collision|GetOverlappingActors (Variables|Default|GetObjects) "/Game/Blueprints/destrutible.destrutible_C" :!class /Script/Engine.PrimitiveComponent)
    (bind _asdestrutible (Utilities|Casting|CastTodestrutible _array_element))
    (Utilities|Array|Add (Variables|Default|GetdestrcutionArray) _asdestrutible)
    (Variables|/Game/Blueprints/destrutible.destrutible_C|SetdestructionCam _asdestrutible self))
  (Components|DestroyComponent (Variables|Default|GetObjects))
  (bind _returnvalue (Class|GameplayStatics|GetActorArrayAverageLocation (Variables|Default|GetdestrcutionArray)))
  (Transformation|SetWorldLocation (Variables|Default|GetDefaultSceneRoot) _returnvalue false false))

(event EventBeginPlay
  (if (== (Utilities|Array|Length (Variables|Default|GetdestrcutionArray)) 0)
    (Utilities|FlowControl|Delay 0.0)
    (CallFunction|PopulateArray)))

(event Collision|EventActorBeginOverlap
  (params (OtherActor :type Actor%20Object%20Reference)))

(event EventTick
  (params (DeltaSeconds :type Float%20%28single-precision%29)))

(fn ConstructionScript)