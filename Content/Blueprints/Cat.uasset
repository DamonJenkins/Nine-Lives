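; Physics-driven cat with a limited pool of lives that ends the game by opening EndScreen.
; Attract and Repel each spend a life to push CatBody toward or away from a point with a meow; Attract pushes only horizontally.
; Impacts above HurtThreshold also cost a life, spawning smoke or ending the game if none remain.
; Tick also ends the game once a lifeless cat stays nearly still for a few seconds.
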(event Custom|Attract
  (params (World%20Location :type Vector) (Magnitude :type Float%20%28single-precision%29))
  (bind _lives (Variables|Default|GetLives))
  (bind _catbody (Variables|Default|GetCatBody))
  (bind _returnvalue (Transformation|GetWorldLocation _catbody))
  (bind _returnvalue_2 (- World%20Location (Math|Vector|MakeVector (.x _returnvalue) (.y _returnvalue) 0.0)))
  (if (not (== _lives 0))
    (Math|Integer|DecrementInt _lives
      (:%20%20
        (Physics|AddForce (Variables|Default|GetCatBody) (* (Math|Vector|Normalize (Math|Vector|MakeVector (.x _returnvalue_2) (.y _returnvalue_2) 0.0)) Magnitude) "None" false)
        (Audio|PlaySoundatLocation "/Game/Sounds/Meow.Meow" (Transformation|GetWorldLocation (Variables|Default|GetCatBody)) "0, 0, 0" 1.0 1.0 0.0 0 0 0)))))

(event Custom|Repel
  (params (World%20Location :type Vector) (Magnitude :type Float%20%28single-precision%29))
  (bind _lives (Variables|Default|GetLives))
  (bind _catbody (Variables|Default|GetCatBody))
  (if (not (== _lives 0))
    (Math|Integer|DecrementInt _lives
      (:%20%20
        (Physics|AddForce _catbody (* (Math|Vector|Normalize (- (Transformation|GetWorldLocation _catbody) World%20Location)) Magnitude) "None" false)
        (Audio|PlaySoundatLocation "/Game/Sounds/Meow.Meow" (Transformation|GetWorldLocation (Variables|Default|GetCatBody)) "0, 0, 0" 1.0 1.0 0.0 0 0 0)))))

(event EventBeginPlay)

(event Collision|EventActorBeginOverlap
  (params (OtherActor :type Actor%20Object%20Reference)))

(event EventTick
  (params (DeltaSeconds :type Float%20%28single-precision%29))
  (if (== (Variables|Default|GetLives) 0)
    (if (< (Transformation|GetVelocity) 0.1)
      (bind _output_get (Variables|Default|SetStoppedMovingTimer (+ (Variables|Default|GetStoppedMovingTimer) DeltaSeconds)))
      (if (> _output_get 3.0)
        (Game|OpenLevel(byName) "EndScreen"))
      (else
        (Variables|Default|SetStoppedMovingTimer 0.0)))))

(event Collision|EventHit
  (params (MyComp :type Primitive%20Component%20Object%20Reference) (Other :type Actor%20Object%20Reference) (OtherComp :type Primitive%20Component%20Object%20Reference) (bSelfMoved :type Boolean) (HitLocation :type Vector :default "0, 0, 0") (HitNormal :type Vector :default "0, 0, 0") (NormalImpulse :type Vector :default "0, 0, 0") (Hit :type Hit%20Result%20Structure%20%28by%20ref%29))
  (if (> (Math|Vector|VectorLength NormalImpulse) (Variables|Default|GetHurtThreshold))
    (bind _result (Math|Integer|DecrementInt (Variables|Default|GetLives))
      (:%20%20
        ;[1 1 1] Close Game Loop
        (if (<= _result 0)
          (Game|OpenLevel(byName) "EndScreen")
          (else
            (Effects|SpawnEmitteratLocation "/Game/Assets/Particle_Systems/P_Smoke_Impact.P_Smoke_Impact" HitLocation)))))))

(fn ConstructionScript)